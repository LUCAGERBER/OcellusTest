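; BP_FeedbackManager plays the completion feedback when the dog's wound has been cleaned.
; After a short deferral at BeginPlay it binds to the wound's OnCleaned event and caches the camera's start position.
; On completion it plays success and happy-bark sounds, releases the pliers and spawns a Niagara effect at the wound.
; A timeline then bumps the camera along its forward vector from the cached position.
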(event Custom|CleaningCompleted
  (Audio|PlaySound2D "/Game/SFX/SFX_Complete.SFX_Complete" 1.0 1.0 0.0 0 0)
  (Audio|PlaySound2D "/Game/SFX/SFX_HappyBark.SFX_HappyBark" 1.0 1.0 0.0 0 0)
  (Variables|/Game/3D/Tools/BP_Tool.BP_Tool_C|SetisHeld (Variables|Default|GetpliersRef) false)
  (Niagara|SpawnSystematLocation "/Game/Particle/NS_CleaningCompleted.NS_CleaningCompleted" (Transformation|GetActorLocation (Variables|/Game/3D/Dog/Medium_Dog/BP_Dog.BP_Dog_C|Getwound (Variables|Default|GetdogRef))) "45.000000,0.000000,0.000000")
  (bind _time (Timeline|CameraBump PlayFromStart)
    (:Update
      (Transformation|SetActorLocation (Variables|Default|GetcamRef) (+ (Variables|Default|GetcameraStartPos) (* (* _time (Variables|Default|GetbumpStrength)) (Transformation|GetActorForwardVector (Variables|Default|GetcamRef)))) false false))))

(event EventBeginPlay
  (Utilities|FlowControl|Delay 0.0)
  (EventDispatchers|BindEventtoOnCleaned (Variables|/Game/3D/Dog/Medium_Dog/BP_Dog.BP_Dog_C|Getwound (Variables|Default|GetdogRef)) (delegate Custom|CleaningCompleted))
  (Variables|Default|SetcameraStartPos (Transformation|GetActorLocation (Variables|Default|GetcamRef))))

(fn ConstructionScript)
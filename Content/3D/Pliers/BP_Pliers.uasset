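; Pliers tool that can be hovered and held, with a yaw sway as it is moved while held.
; It passes hover and hold events to its parent class, supplying its box collider, and creates a dynamic overlay material on the skeletal mesh.
; Half a second after a held event it caches a base rotation.
; Tick then turns per-frame X movement into a clamped, interpolated yaw offset from that rotation.
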(event EventTick
  (params (DeltaSeconds :type Float%20%28single-precision%29))
  (bind _tiltamount (Variables|Default|GettiltAmount))
  (if (and (Variables|Default|GetisHeld) (Variables|Default|GetbaseRotSet))
    (Variables|Default|SetcurrentLocation (Transformation|GetActorLocation))
    (Variables|Default|SetmovementDelta (- (Variables|Default|GetcurrentLocation) (Variables|Default|GetpreviousLocation)))
    (Variables|Default|SetpreviousLocation (Variables|Default|GetcurrentLocation))
    (Variables|Default|SettargetTilt (Math|Float|Clamp(Float) (* (.x (Variables|Default|GetmovementDelta)) (Variables|Default|GettiltSensitivy)) (* _tiltamount -1.0) _tiltamount))
    (Variables|Default|SetcurrentTilt (Math|Interpolation|FInterpTo (Variables|Default|GetcurrentTilt) (Variables|Default|GettargetTilt) DeltaSeconds (Variables|Default|GettiltInterpSpeed)))
    (Transformation|SetActorRotation (Math|Rotator|CombineRotators (Variables|Default|GetbaseRot) (Math|Rotator|MakeRotator 0.0 0.0 (Variables|Default|GetcurrentTilt))))))

(event EventBeginPlay
  (|CallParentFunction)
  (Variables|Default|SetmyCollider (Variables|Default|GetBox_Collider))
  (CallFunction|CreateDynOverlayMaterial (Variables|Default|GetSK_Pliers)))

(event EventOnHover
  (params (IsHover :type Boolean))
  (|CallParentFunction IsHover))

(event EventOnHeld
  (params (held :type Boolean) (collider :type Primitive%20Component%20Object%20Reference))
  (|CallParentFunction held (Variables|Default|GetBox_Collider))
  (Variables|Default|SetpreviousLocation (Transformation|GetActorLocation))
  (Utilities|FlowControl|Delay 0.5)
  (Variables|Default|SetbaseRot (Transformation|GetActorRotation))
  (Variables|Default|SetbaseRotSet true))

(fn ConstructionScript)
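; BP_Dog is a medium dog actor with a wound that can be cleaned.
; On BeginPlay it spawns BP_Wound, attaches it to a socket on the dog's skeletal mesh and listens for its cleaned event.
; While Cry is set, Tick plays cry sounds at randomized intervals.
; Cleaning the wound stops the crying, flags the dog's animation blueprint to react and starts a happy breathing sound.
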(event Custom|OnWoundCleaned
  (bind _asabp_dog (Utilities|Casting|CastToABP_Dog (Components|SkeletalMesh|GetAnimInstance (Variables|Default|GetSK_Dog_Medium))))
  (Variables|/Game/3D/Dog/Medium_Dog/Animations/ABP_Dog.ABP_Dog_C|SetshouldReact _asabp_dog true)
  (Variables|Default|Setcry false)
  (bind _returnvalue (Audio|SpawnSound2D "/Game/SFX/SFX_Dog_HappyBreathing.SFX_Dog_HappyBreathing" 1.0 1.0 0.0 0))
  (Variables|Default|SetdogBreath _returnvalue))

(event EventBeginPlay
  (bind _returnvalue (Game|SpawnActorfromClass "/Game/3D/Dog/Medium_Dog/BP_Wound.BP_Wound_C" (Math|Transform|MakeTransform "0, 0, 0" "0, 0, 0" "1.000000,1.000000,1.000000") "Undefined" "MultiplyWithRoot" 0 0))
  (bind _output_get (Variables|Default|Setwound _returnvalue))
  (Transformation|AttachComponentToComponent _output_get (Variables|Default|GetSK_Dog_Medium) "Wound_Socket_1" "SnapToTarget" "SnapToTarget" "KeepWorld" true)
  (EventDispatchers|BindEventtoOnCleaned (Variables|Default|Getwound) (delegate Custom|OnWoundCleaned)))

(event EventTick
  (params (DeltaSeconds :type Float%20%28single-precision%29))
  (if (and (Variables|Default|Getcry) (>= (Variables|Default|Getelapsed) (Variables|Default|GettimeBetweenCry)))
    (Audio|PlaySound2D "/Game/SFX/SFX_Dog_Cry.SFX_Dog_Cry" 1.0 1.0 0.0 0 0)
    (Variables|Default|Setelapsed 0.0)
    (Variables|Default|SettimeBetweenCry (Math|Random|RandomFloatinRange (Variables|Default|GettimeBetweenCryMin) (Variables|Default|GettimeBetyweenCryMax)))
    (else
      (Variables|Default|Setelapsed (+ DeltaSeconds (Variables|Default|Getelapsed))))))

(fn ConstructionScript)
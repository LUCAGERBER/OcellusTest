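; BP_Wound is a wound decal, filed under the medium dog assets, that is cleaned by moving a BP_Cotton actor inside its box.
; Box overlaps track the cotton, and each tick converts the distance it moved into a reduction of the blood amount.
; That value drives a scalar on the decal's dynamic material, and its inverse is sent to the cotton to display blood progression.
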(event OnComponentBeginOverlap(Box)
  (params (OverlappedComponent :type Primitive%20Component%20Object%20Reference) (OtherActor :type Actor%20Object%20Reference) (OtherComp :type Primitive%20Component%20Object%20Reference) (OtherBodyIndex :type Integer) (bFromSweep :type Boolean) (SweepResult :type Hit%20Result%20Structure%20%28by%20ref%29))
  (bind _asbp_cotton (Utilities|Casting|CastToBP_Cotton OtherActor))
  (Variables|Default|SetisCottonInside true)
  (bind _output_get (Variables|Default|SetcottonRef _asbp_cotton))
  (Variables|Default|SetpreviousCottonLocation (Transformation|GetActorLocation _output_get)))

(event OnComponentEndOverlap(Box)
  (params (OverlappedComponent :type Primitive%20Component%20Object%20Reference) (OtherActor :type Actor%20Object%20Reference) (OtherComp :type Primitive%20Component%20Object%20Reference) (OtherBodyIndex :type Integer))
  (Utilities|Casting|CastToBP_Cotton OtherActor)
  (Variables|Default|SetisCottonInside false)
  (Variables|Default|SetcottonRef 0))

(event EventTick
  (params (DeltaSeconds :type Float%20%28single-precision%29))
  (if (Variables|Default|GetisCottonInside)
    (Variables|Default|SetcurrentCottonLocation (Transformation|GetActorLocation (Variables|Default|GetcottonRef)))
    (Variables|Default|SetdistanceMoved (Math|Vector|Distance(Vector) (Variables|Default|GetcurrentCottonLocation) (Variables|Default|GetpreviousCottonLocation)))
    (Variables|Default|SetpreviousCottonLocation (Variables|Default|GetcurrentCottonLocation))
    (Variables|Default|SetcleanAmount (* (Variables|Default|GetdistanceMoved) (Variables|Default|GetcleaningMultiplier)))
    (bind _output_get (Variables|Default|SetbloodAmount (- (Variables|Default|GetbloodAmount) (Variables|Default|GetcleanAmount))))
    (Rendering|Material|SetScalarParameterValue (Variables|Default|GetdynMaterial) "bloodAmount" _output_get :!class /Script/Engine.MaterialInstanceDynamic)
    (Default|DisplayBloodProgression (Variables|Default|GetcottonRef) (- 1.0 _output_get))))

(event EventBeginPlay
  (bind _returnvalue (Rendering|Material|CreateDynamicMaterialInstance (Variables|Default|GetDecal) :!class /Script/Engine.DecalComponent))
  (bind _output_get (Variables|Default|SetdynMaterial _returnvalue))
  (Rendering|Components|Decal|SetDecalMaterial (Variables|Default|GetDecal) _output_get))

(fn ConstructionScript)
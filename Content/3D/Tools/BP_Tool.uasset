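; BP_Tool is a tool actor, apparently a base, that supports hover highlighting and being held.
; CreateDynOverlayMaterial turns a given mesh's overlay material into a dynamic instance and starts it unhighlighted.
; OnHover toggles that overlay's OutlineThickness parameter and the highlight flag.
; OnHeld calls SetHeld, which stores the held state and, when held, makes the collider ignore Visibility traces, without restoring this on release.
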(event Custom|OnHover
  (params (IsHover :type Boolean))
  (if IsHover
    (Rendering|Material|SetScalarParameterValue (Variables|Default|GetdynOverlayMaterial) "OutlineThickness" (Variables|Default|GetoutlineThickness) :!class /Script/Engine.MaterialInstanceDynamic)
    (Variables|Default|SetisHighlited true)
    (else
      (Rendering|Material|SetScalarParameterValue (Variables|Default|GetdynOverlayMaterial) "OutlineThickness" 0.0 :!class /Script/Engine.MaterialInstanceDynamic)
      (Variables|Default|SetisHighlited false))))

(event Custom|OnHeld
  (params (held :type Boolean) (collider :type Primitive%20Component%20Object%20Reference))
  (CallFunction|SetHeld held collider))

(fn ConstructionScript)

(fn SetHeld
  (params (isHeld :type Boolean) (collider :type Primitive%20Component%20Object%20Reference))
  (bind _output_get (Variables|Default|SetisHeld isHeld))
  (if _output_get
    (Collision|SetCollisionResponsetoChannel collider "ECC_Visibility" "ECR_Ignore")))

(fn CreateDynOverlayMaterial
  (params (mesh :type Mesh%20Component%20Object%20Reference))
  (bind _returnvalue (Rendering|Material|CreateDynamicMaterialInstance (Rendering|Material|GetOverlayMaterial mesh :!class /Script/Engine.MeshComponent) "None" "None" :!class /Script/Engine.KismetMaterialLibrary))
  (bind _output_get (Variables|Default|SetdynOverlayMaterial _returnvalue))
  (Rendering|Material|SetOverlayMaterial mesh _output_get :!class /Script/Engine.MeshComponent)
  (CallFunction|OnHover false))
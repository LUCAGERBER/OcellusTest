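; BP_Cotton is a holdable cotton prop that deforms when scrubbed and displays blood staining.
; Tick measures distance moved each frame; while scrubbing, it drives a squash-and-stretch mesh scale and the fur scrub Niagara intensity, otherwise resetting both.
; A dynamic material exposes blood progression as a scalar parameter.
; A separate timeline-driven Squash event scales the actor from its base scale, which is re-cached shortly after OnHeld.
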(event Custom|Squash
  (Variables|Default|SettargetScale (+ (Variables|Default|GetbaseScale) (Variables|Default|GetoffsetScale)))
  (bind _tick (Timeline|SquashTimeLine PlayFromStart)
    (:Update
      (Transformation|SetActorScale3D (Math|Vector|Lerp(Vector) (Variables|Default|GetbaseScale) (Variables|Default|GettargetScale) _tick)))))

(event EventTick
  (params (DeltaSeconds :type Float%20%28single-precision%29))
  (CallFunction|CalculateDistanceMoved)
  (if (Variables|Default|GetisScrubbing)
    (CallFunction|ScrubSquash DeltaSeconds)
    (Niagara|SetNiagaraVariable(Float) (Variables|Default|GetNS_FurScrub) "scrubIntensity" (Variables|Default|GetdistanceMoved))
    (else
      (Niagara|SetNiagaraVariable(Float) (Variables|Default|GetNS_FurScrub) "scrubIntensity" 0.0)
      (Transformation|SetWorldScale3D (Variables|Default|GetSM_Cotton) "1.000000,1.000000,1.000000"))))

(event EventBeginPlay
  (|CallParentFunction)
  (CallFunction|CreateDynOverlayMaterial (Variables|Default|GetSM_Cotton))
  (bind _returnvalue (Rendering|Material|CreateDynamicMaterialInstance (Variables|Default|GetSM_Cotton) 0 "/Game/3D/Cotton/M_Cotton.M_Cotton" "None" :!class /Script/Engine.PrimitiveComponent))
  (Variables|Default|SetdynMat _returnvalue)
  (Rendering|Material|SetMaterial (Variables|Default|GetSM_Cotton) 0 (Variables|Default|GetdynMat))
  (Variables|Default|SetbaseScale (Transformation|GetActorScale3D))
  (Niagara|SetNiagaraVariable(Float) (Variables|Default|GetNS_FurScrub) "scrubIntensity" 0.0))

(event EventOnHeld
  (params (held :type Boolean) (collider :type Primitive%20Component%20Object%20Reference))
  (|CallParentFunction held (Variables|Default|GetSphere))
  (Utilities|FlowControl|Delay 0.2)
  (Variables|Default|SetbaseScale (Transformation|GetActorScale3D)))

(fn ConstructionScript)

(fn DisplayBloodProgression
  (params (bloodAmount :type Float%20%28double-precision%29))
  (Rendering|Material|SetScalarParameterValue (Variables|Default|GetdynMat) "bloodStain" bloodAmount :!class /Script/Engine.MaterialInstanceDynamic))

(fn GetDistanceMoved
  (return (Variables|Default|GetdistanceMoved)))

(fn CalculateDistanceMoved
  (Variables|Default|SetcurrentLocation (Transformation|GetActorLocation))
  (Variables|Default|SetdistanceMoved (Math|Vector|Distance(Vector) (Variables|Default|GetcurrentLocation) (Variables|Default|GetpreviousLocation)))
  (Variables|Default|SetpreviousLocation (Variables|Default|GetcurrentLocation)))

(fn ScrubSquash
  (params (InputPin :type Float%20%28single-precision%29))
  (bind _distancemoved (Variables|Default|GetdistanceMoved))
  (bind _scrubintensity (Variables|Default|GetscrubIntensity))
  (bind _returnvalue (Math|Float|Clamp(Float) _distancemoved))
  (bind _returnvalue_2 (+ _returnvalue 1.0))
  (bind _returnvalue_3 (* _returnvalue_2 _scrubintensity))
  (Transformation|SetWorldScale3D (Variables|Default|GetSM_Cotton) (Math|Interpolation|VInterpTo (Variables|Default|GetbaseScale) (* (Variables|Default|GetbaseScale) (Math|Vector|MakeVector _returnvalue_3 (* (- 1.0 _returnvalue) _scrubintensity) _returnvalue_3)) InputPin 12.0)))